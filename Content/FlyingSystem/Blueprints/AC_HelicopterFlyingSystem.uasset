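; Helicopter flight component that moves and tilts its owner each tick while flying logic is enabled.
; Input functions set camera-relative direction, target roll, pitch and yaw, and vertical state.
; Fly eases mesh rotations toward those targets and accelerates or slows horizontal and vertical speeds, with boosting.
; Curves for heading-to-travel angle, remaining power and carried weight scale horizontal speed; vertical movement applies the unscaled speed despite computing a scaled one.
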(event `self.ReceiveTick`
  (params (DeltaSeconds :type "Float (single-precision)"))
  (if (`self.EnabledFlyingLogic`)
    (`self.Fly`)))

(fn `AddHorizontalInput`
  (params (Direction :type "Vector2D Structure"))
  (bind (_returnvalue_x _returnvalue_y) (`KismetMathLibrary.BreakVector2D` (`KismetMathLibrary.Normal2D` Direction)))
  (bind _springarmlocalreferencearrow (`self.SpringArmLocalReferenceArrow`))
  (bind (_returnvalue_roll _returnvalue_pitch _returnvalue_yaw) (`KismetMathLibrary.BreakRotator` (`SceneComponent.K2_GetComponentRotation` (`self.RollRoot`))))
  (bind (_returnvalue_roll_2 _returnvalue_pitch_2 _returnvalue_yaw_2) (`KismetMathLibrary.BreakRotator` (`SceneComponent.K2_GetComponentRotation` (`self.SpringArm`))))
  (bind _returnvalue (* (`self.MaximumMeshPitchAngle`) _returnvalue_y))
  (bind _returnvalue_2 (* (`self.MaximumMeshRollAngle`) _returnvalue_x))
  (set `self.HorizontalMoving` true)
  (if (< (`self.DeltaAngle` _returnvalue_yaw_2 _returnvalue_yaw) 90.0)
    (set `self.TargetMeshLocalRotationX` _returnvalue_2)
    (set `self.TargetMeshLocalRotationY` (* _returnvalue -1.0))
    (else
      (set `self.TargetMeshLocalRotationX` (* _returnvalue_2 -1.0))
      (set `self.TargetMeshLocalRotationY` _returnvalue)))
  (`SceneComponent.K2_SetRelativeLocation` _springarmlocalreferencearrow (`KismetMathLibrary.MakeVector` (* _returnvalue_y 1000000.0) (* _returnvalue_x 1000000.0)) false false)
  (bind _output_get (set `self.FlyingDirection` (- (`SceneComponent.K2_GetComponentLocation` _springarmlocalreferencearrow) (`SceneComponent.K2_GetComponentLocation` (`self.SceneRoot`)))))
  (set `self.FlyingDirection` (`KismetMathLibrary.Normal` (`KismetMathLibrary.MakeVector` (.x _output_get) (.y _output_get)))))

(fn `AddVerticalInput`
  (params (Value :type "Float (double-precision)"))
  (set `self.VerticalMoving` true)
  (set `self.VerticalSlowingDown` false)
  (if (> Value 0.01)
    (set `self.Ascending` true)
    (else
      (set `self.Ascending` false))))

(fn `AddWeight`
  (params (IncreaseValue :type "Float (double-precision)"))
  (bind _maximumcarryingweight (`self.MaximumCarryingWeight`))
  (set `self.CurrentCarryingWeight` (`KismetMathLibrary.FClamp` (+ (`self.CurrentCarryingWeight`) 1.0) 0.0 _maximumcarryingweight))
  (set `self.WeightPercentage` (/ (`self.WeightPercentage`) _maximumcarryingweight)))

(fn `AddYawInput`
  (params (Value :type "Float (double-precision)"))
  (set `self.TargetMeshLocalRotationZ` (+ (`self.TargetMeshLocalRotationZ`) (* Value (`self.MeshYawTurningSpeed`) (`GameplayStatics.GetWorldDeltaSeconds`)))))

(fn `DeltaAngle`
  (params (Angle1 :type "Float (double-precision)") (Angle2 :type "Float (double-precision)"))
  (returns (Angle :type "Float (double-precision)"))
  (bind _newangle1 (`self.NewAngle1`))
  (bind _newangle2 (`self.NewAngle2`))
  (if (< Angle1 0.0)
    (set `self.NewAngle1` (+ Angle1 360.0))
    (else
      (set `self.NewAngle1` Angle1)))
  (if (< Angle2 0.0)
    (set `self.NewAngle2` (+ Angle2 360.0))
    (else
      (set `self.NewAngle2` Angle2)))
  (if (and (> _newangle1 270.0) (< _newangle2 90.0))
    (return (- (+ _newangle2 360.0) _newangle1))
    (elif (and (< _newangle1 90.0) (> _newangle2 270.0))
      (return (- (+ _newangle1 360.0) _newangle2))
      (else
        (return (`KismetMathLibrary.Abs` (- _newangle2 _newangle1)))))))

(fn `Fly`
  (bind _returnvalue (`GameplayStatics.GetWorldDeltaSeconds`))
  (bind _returnvalue_2 (`GameplayStatics.GetWorldDeltaSeconds`))
  (bind _returnvalue_3 (`GameplayStatics.GetWorldDeltaSeconds`))
  (bind (_flyingdirection_x _flyingdirection_y) (`KismetMathLibrary.BreakVector` (`self.FlyingDirection`)))
  (bind _rollroot (`self.RollRoot`))
  (bind _rollroot_2 (`self.RollRoot`))
  (bind _currenthorizontalflyingspeed (`self.CurrentHorizontalFlyingSpeed`))
  (bind _normalhorizontalflyingspeed (`self.NormalHorizontalFlyingSpeed`))
  (bind _sceneroot (`self.SceneRoot`))
  (bind _boosting (`self.Boosting`))
  (bind _currentverticalflyingspeed (`self.CurrentVerticalFlyingSpeed`))
  (bind _maximumverticalflyingspeed (`self.MaximumVerticalFlyingSpeed`))
  (bind _currentverticalflyingspeed_2 (`self.CurrentVerticalFlyingSpeed`))
  (bind _normalverticalflyingspeed (`self.NormalVerticalFlyingSpeed`))
  (bind _sceneroot_2 (`self.SceneRoot`))
  (bind _currentverticalflyingspeed_3 (`self.CurrentVerticalFlyingSpeed`))
  (bind _meshroot (`self.MeshRoot`))
  (bind _maximumpower (`self.MaximumPower`))
  (bind _currentpower (`self.CurrentPower`))
  (bind (_returnvalue_x _returnvalue_y) (`KismetMathLibrary.BreakVector` (`SceneComponent.GetForwardVector` (`self.MeshRoot`))))
  (bind _returnvalue_4 (* (`self.MeshPitchTurningSmoothingFactor`) _returnvalue_3))
  (bind _returnvalue_5 (* (`self.VerticalBoostAcceleration`) (`GameplayStatics.GetWorldDeltaSeconds`)))
  (bind _returnvalue_6 (* _maximumverticalflyingspeed -1.0))
  (bind _returnvalue_7 (* _normalverticalflyingspeed -1.0))
  (bind _returnvalue_8 (* (`self.HorizontalBoostAcceleration`) _returnvalue_2))
  (bind _returnvalue_9 (* (`self.MeshRollTurningSmoothingFactor`) _returnvalue_3))
  (bind (_relativerotation_roll _relativerotation_pitch _relativerotation_yaw) (`KismetMathLibrary.BreakRotator` (`SceneComponent.RelativeRotation` _rollroot)))
  (bind (_relativerotation_roll_2 _relativerotation_pitch_2) (`KismetMathLibrary.BreakRotator` (`SceneComponent.RelativeRotation` _meshroot)))
  (bind (_relativerotation_roll_3 _relativerotation_pitch_3 _relativerotation_yaw_2) (`KismetMathLibrary.BreakRotator` (`SceneComponent.RelativeRotation` _rollroot_2)))
  (bind _returnvalue_10 (- _currentverticalflyingspeed_2 _returnvalue_5))
  (bind _returnvalue_11 (+ (`self.CurrentHorizontalFlyingSpeed`) _returnvalue_8))
  (`SceneComponent.K2_SetRelativeRotation` _rollroot (`KismetMathLibrary.RLerp` (`KismetMathLibrary.MakeRotator` _relativerotation_roll 0.0 _relativerotation_yaw) (`KismetMathLibrary.MakeRotator` _relativerotation_roll 0.0 (`self.TargetMeshLocalRotationZ`)) (* (`self.MeshYawTurningSmoothingFactor`) (`GameplayStatics.GetWorldDeltaSeconds`)) true) false false)
  (set `self.AngleFactor` (`CurveFloat.GetFloatValue` (`self.SpeedTailRotorAngleRatioCurve`) (/ (`KismetMathLibrary.DegAcos` (`KismetMathLibrary.Dot_VectorVector` (`KismetMathLibrary.Normal` (`KismetMathLibrary.MakeVector` _flyingdirection_x _flyingdirection_y)) (`KismetMathLibrary.Normal` (`KismetMathLibrary.MakeVector` _returnvalue_x _returnvalue_y)))) 180.0)))
  ;[1 1 1] Power Consumption
  (if (`self.CalculatePowerConsumption`)
    (if (`self.InAir`)
      (if (`self.Boosting`)
        (set `self.CurrentPower` (`KismetMathLibrary.FClamp` (- _currentpower (* (`self.PowerDecreaseSpeed`) _returnvalue)) 0.0 _maximumpower))
        (else
          (set `self.CurrentPower` (`KismetMathLibrary.FClamp` (- _currentpower (* (`self.PowerDecreaseSpeedWhenBoosting`) _returnvalue)) 0.0 _maximumpower))))
      (bind _output_get (set `self.PowerPercentage` (/ (`self.CurrentPower`) _maximumpower)))
      (set `self.PowerFactor` (`CurveFloat.GetFloatValue` (`self.SpeedRemainingPowerRatioCurve`) (- 1.0 _output_get)))
      ;[1 1 1] Carrying Weight
      (if (`self.CalculateCarryingWeight`) :!label _label
        (bind _output_get_2 (set `self.WeightPercentage` (/ (`self.CurrentCarryingWeight`) (`self.MaximumCarryingWeight`))))
        (set `self.WeightFactor` (`CurveFloat.GetFloatValue` (`self.SpeedCarryingWeightRatioCurve`) _output_get_2))
        (else
          (set `self.WeightFactor` 1.0)))
      (if (`self.HorizontalMoving`)
        (`SceneComponent.K2_SetRelativeRotation` _rollroot_2 (`KismetMathLibrary.RLerp` (`KismetMathLibrary.MakeRotator` _relativerotation_roll_3 0.0 _relativerotation_yaw_2) (`KismetMathLibrary.MakeRotator` (`self.TargetMeshLocalRotationX`) 25.0 _relativerotation_yaw_2) _returnvalue_9 true) false false)
        (`SceneComponent.K2_SetRelativeRotation` _meshroot (`KismetMathLibrary.MakeRotator` 0.0 (`KismetMathLibrary.Lerp` _relativerotation_pitch_2 (`self.TargetMeshLocalRotationY`) _returnvalue_4)) false false)
        (if (`self.Boosting`)
          (set `self.CurrentHorizontalFlyingSpeed` (`KismetMathLibrary.FClamp` _returnvalue_11 0.0 (`self.MaximumHorizontalFlyingSpeed`)))
          (elif (> _currenthorizontalflyingspeed _normalhorizontalflyingspeed)
            (set `self.CurrentHorizontalFlyingSpeed` (- _currenthorizontalflyingspeed _returnvalue_8))
            (else
              (set `self.CurrentHorizontalFlyingSpeed` (`KismetMathLibrary.FClamp` _returnvalue_11 0.0 _normalhorizontalflyingspeed)))))
        (else
          (`SceneComponent.K2_SetRelativeRotation` _rollroot_2 (`KismetMathLibrary.RLerp` (`KismetMathLibrary.MakeRotator` _relativerotation_roll_3 _relativerotation_pitch_3 _relativerotation_yaw_2) (`KismetMathLibrary.MakeRotator` 0.0 0.0 _relativerotation_yaw_2) _returnvalue_9 true) false false)
          (`SceneComponent.K2_SetRelativeRotation` _meshroot (`KismetMathLibrary.MakeRotator` 0.0 (`KismetMathLibrary.Lerp` _relativerotation_pitch_2 0.0 _returnvalue_4)) false false)
          (set `self.CurrentHorizontalFlyingSpeed` (`KismetMathLibrary.FClamp` (- _currenthorizontalflyingspeed (* (`self.HorizontalSlowDownAcceleration`) _returnvalue_2)) 0.0 _normalhorizontalflyingspeed))))
      (set `self.HorizontalFlyingSpeed` (* (`self.CurrentHorizontalFlyingSpeed`) (`self.AngleFactor`) (`self.PowerFactor`) (`self.WeightFactor`)))
      (`SceneComponent.K2_SetWorldLocation` _sceneroot_2 (+ (`SceneComponent.K2_GetComponentLocation` _sceneroot_2) (* (`self.FlyingDirection`) (* (`self.HorizontalFlyingSpeed`) _returnvalue_2))) false false)
      (if (`self.VerticalMoving`)
        (if (`self.Ascending`)
          (if _boosting
            (set `self.CurrentVerticalFlyingSpeed` (`KismetMathLibrary.FClamp` (+ _currentverticalflyingspeed _returnvalue_5) 0.0 _maximumverticalflyingspeed))
            (elif (> _currentverticalflyingspeed_2 _normalverticalflyingspeed)
              (set `self.CurrentVerticalFlyingSpeed` (- _currentverticalflyingspeed _returnvalue_5))
              (else
                (set `self.CurrentVerticalFlyingSpeed` (`KismetMathLibrary.FClamp` (+ _currentverticalflyingspeed_2 _returnvalue_5) 0.0 _maximumverticalflyingspeed)))))
          (elif _boosting
            (set `self.CurrentVerticalFlyingSpeed` (`KismetMathLibrary.FClamp` (- _currentverticalflyingspeed_2 _returnvalue_5) _returnvalue_6 _maximumverticalflyingspeed))
            (elif (< _currentverticalflyingspeed_2 _returnvalue_7)
              (set `self.CurrentVerticalFlyingSpeed` (+ _currentverticalflyingspeed_2 _returnvalue_5))
              (else
                (set `self.CurrentVerticalFlyingSpeed` (`KismetMathLibrary.FClamp` _returnvalue_10 _returnvalue_7 _normalverticalflyingspeed))))))
        (set `self.VerticalFlyingSpeed` (* (`self.CurrentVerticalFlyingSpeed`) (`self.PowerFactor`) (`self.WeightFactor`)) :!label _label_2)
        (`SceneComponent.K2_SetWorldLocation` _sceneroot (+ (`SceneComponent.K2_GetComponentLocation` _sceneroot) (`KismetMathLibrary.MakeVector` 0.0 0.0 (* (`self.CurrentVerticalFlyingSpeed`) (`GameplayStatics.GetWorldDeltaSeconds`)))) false false)
        (elif (`self.VerticalSlowingDown`)
          (if (< _currentverticalflyingspeed_3 0.0)
            (set `self.CurrentVerticalFlyingSpeed` (`KismetMathLibrary.FClamp` (+ _currentverticalflyingspeed_3 _returnvalue_5) _returnvalue_6 0.0))
            (goto _label_2)
            (else
              (set `self.CurrentVerticalFlyingSpeed` (`KismetMathLibrary.FClamp` _returnvalue_10 0.0 _maximumverticalflyingspeed))
              (goto _label_2))))))
    (else
      (set `self.PowerFactor` 1.0)
      (goto _label))))

(fn `Land`
  (set `self.InAir` false))

(fn `StopYawInput`
  (set `self.HorizontalMoving` false))

(fn `TakeOff`
  (set `self.InAir` true))

(fn `VerticalSlowDown`
  (set `self.VerticalMoving` false)
  (set `self.VerticalSlowingDown` true))
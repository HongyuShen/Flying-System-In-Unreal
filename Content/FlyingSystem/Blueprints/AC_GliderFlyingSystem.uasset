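; Glider flight component that, while airborne, moves the owner's SceneRoot kinematically each tick without sweep or physics simulation.
; Yaw, pitch and roll inputs set clamped targets that MeshRoot eases toward, with roll plus yaw also turning SceneRoot.
; MeshRoot's forward vector drives velocity, scaled by an optional carried-weight curve.
; Gravity and pitch-dependent drag cause sinking, steep dives build speed that later decays, and airflow zones add fading lift.
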(event `self.ReceiveTick`
  (params (DeltaSeconds :type "Float (single-precision)"))
  (if (`self.EnabledFlyingLogic`)
    (`self.Fly`)))

(fn `AddAirflowForce`
  (params (Intensity :type "Float (double-precision)") (Acceleration :type "Float (double-precision)") (FadeOutAcceleration :type "Float (double-precision)"))
  (set `self.AirflowIntensity` Intensity)
  (set `self.AirflowAcceleration` Acceleration)
  (set `self.AirflowFadeOutAcceleration` FadeOutAcceleration)
  (set `self.TargetMeshLocalRotationY` (`KismetMathLibrary.FClamp` (+ (`self.TargetMeshLocalRotationY`) (`self.LookUpAngle`)) -89.995003 89.995003))
  (set `self.InAirflow` true))

(fn `AddPitchInput`
  (params (Value :type "Float (double-precision)"))
  (set `self.TargetMeshLocalRotationY` (`KismetMathLibrary.FClamp` (+ (`self.TargetMeshLocalRotationY`) (* Value (`self.MeshPitchTurningSpeed`) (`GameplayStatics.GetWorldDeltaSeconds`))) -89.995003 89.995003)))

(fn `AddRollInput`
  (params (Value :type "Float (double-precision)"))
  (bind _maximummeshrollangle (`self.MaximumMeshRollAngle`))
  (set `self.TargetMeshLocalRotationX` (`KismetMathLibrary.FClamp` (+ (`self.TargetMeshLocalRotationX`) (* Value (`self.MeshRollTurningSpeed`) (`GameplayStatics.GetWorldDeltaSeconds`))) (* _maximummeshrollangle -1.0) _maximummeshrollangle)))

(fn `AddWeight`
  (params (IncreaseValue :type "Float (double-precision)"))
  (bind _maximumcarryingweight (`self.MaximumCarryingWeight`))
  (set `self.CurrentCarryingWeight` (`KismetMathLibrary.FClamp` (+ (`self.CurrentCarryingWeight`) IncreaseValue) 0.0 _maximumcarryingweight))
  (set `self.WeightPercentage` (/ (`self.WeightPercentage`) _maximumcarryingweight)))

(fn `AddYawInput`
  (params (Value :type "Float (double-precision)"))
  (bind _maximummeshyawangle (`self.MaximumMeshYawAngle`))
  (set `self.TargetMeshLocalRotationZ` (`KismetMathLibrary.FClamp` (+ (`self.TargetMeshLocalRotationZ`) (* Value (`self.MeshYawTurningSpeed`) (`GameplayStatics.GetWorldDeltaSeconds`))) (* _maximummeshyawangle -1.0) _maximummeshyawangle)))

(fn `EndAirflowForce`
  (set `self.InAirflow` false))

(fn `Fly`
  (bind _returnvalue (`GameplayStatics.GetWorldDeltaSeconds`))
  (bind _returnvalue_2 (`GameplayStatics.GetWorldDeltaSeconds`))
  (bind _returnvalue_3 (`GameplayStatics.GetWorldDeltaSeconds`))
  (bind _returnvalue_4 (`GameplayStatics.GetWorldDeltaSeconds`))
  (bind _currentflyingspeed (`self.CurrentFlyingSpeed`))
  (bind _meshroot (`self.MeshRoot`))
  (bind _decelerationafterdiving (`self.DecelerationAfterDiving`))
  (bind _sceneroot (`self.SceneRoot`))
  (bind (_flyingdirection_x _flyingdirection_y _flyingdirection_z) (`KismetMathLibrary.BreakVector` (`self.FlyingDirection`)))
  (bind _airflowspeed (`self.AirflowSpeed`))
  (bind _sceneroot_2 (`self.SceneRoot`))
  (bind _airflowspeed_2 (`self.AirflowSpeed`))
  (bind _verticalspeed (`self.VerticalSpeed`))
  (bind _sceneroot_3 (`self.SceneRoot`))
  (bind _currentflyingspeed_2 (`self.CurrentFlyingSpeed`))
  (bind _returnvalue_5 (> _currentflyingspeed_2 (`self.OriginalFlyingSpeed`)))
  (bind (_returnvalue_roll _returnvalue_pitch _returnvalue_yaw) (`KismetMathLibrary.BreakRotator` (`SceneComponent.K2_GetComponentRotation` _sceneroot)))
  (bind _returnvalue_6 (`SceneComponent.K2_GetComponentLocation` _sceneroot_3))
  (bind (_relativerotation_roll _relativerotation_pitch _relativerotation_yaw) (`KismetMathLibrary.BreakRotator` (`SceneComponent.RelativeRotation` _meshroot)))
  (bind _returnvalue_7 (* _relativerotation_pitch -1.0))
  (bind _returnvalue_8 (`KismetMathLibrary.FClamp` (- (* (`self.VerticalSpeed`) _returnvalue_2) (* 0.5 (`self.VerticalAcceleration`) _returnvalue_2 _returnvalue_2)) -100000000.0 0.0))
  (if (`self.InAir`)
    ;[1 1 1] Rotation
    (`SceneComponent.K2_SetRelativeRotation` _meshroot (`KismetMathLibrary.MakeRotator` (`KismetMathLibrary.Lerp` _relativerotation_roll (`self.TargetMeshLocalRotationX`) (* (`self.MeshRollTurningSmoothingFactor`) _returnvalue_4)) (`KismetMathLibrary.Lerp` _relativerotation_pitch (`self.TargetMeshLocalRotationY`) (* (`self.MeshPitchTurningSmoothingFactor`) _returnvalue_4)) (`KismetMathLibrary.Lerp` _relativerotation_yaw (`self.TargetMeshLocalRotationZ`) (* (`self.MeshYawTurningSmoothingFactor`) _returnvalue_4))) false false)
    (if (and (not (`self.InAirflow`)) (`self.CanDive`))
      ;[1 1 1] Diving
      (if (> _returnvalue_7 (`self.DivingStartAngle`))
        (if (not (`self.Diving`))
          (set `self.Diving` true)
          (set `self.OriginalFlyingSpeed` _currentflyingspeed))
        (set `self.CurrentFlyingSpeed` (`KismetMathLibrary.FClamp` (+ _currentflyingspeed (* (`self.G`) (`KismetMathLibrary.DegSin` _returnvalue_7) _returnvalue)) 0.0 (`self.MaximumDivingSpeed`)))
        (else
          (set `self.Diving` false)
          (if (< _verticalspeed -0.1)
            (set `self.VerticalSpeed` (+ _verticalspeed (* (`self.AirDrag`) (`KismetMathLibrary.DegCos` _returnvalue_7) _returnvalue)))
            (else
              (set `self.VerticalSpeed` 0.0)))
          ;[1 1 1] Deceleration After Diving
          (if (`KismetMathLibrary.InRange_FloatFloat` _relativerotation_pitch 0.0 -90.0 false false)
            (if _returnvalue_5
              (set `self.CurrentFlyingSpeed` (- _currentflyingspeed_2 (* (+ _decelerationafterdiving (* _decelerationafterdiving (`KismetMathLibrary.DegSin` _returnvalue_7))) _returnvalue)))))
          (if _returnvalue_5
            (set `self.CurrentFlyingSpeed` (- _currentflyingspeed_2 (* _decelerationafterdiving _returnvalue)))))))
    ;[1 1 1] Carrying Weight
    (if (`self.CalculateCarryingWeight`)
      (bind _output_get (set `self.WeightPercentage` (/ (`self.CurrentCarryingWeight`) (`self.MaximumCarryingWeight`))))
      (set `self.WeightFactor` (`CurveFloat.GetFloatValue` (`self.SpeedCarryingWeightRatioCurve`) _output_get))
      (else
        (set `self.WeightFactor` 1.0)))
    (bind _output_get_2 (set `self.FlyingDirection` (`SceneComponent.GetForwardVector` (`self.MeshRoot`))))
    (bind _output_get_3 (set `self.FlyingSpeed` (* (`self.CurrentFlyingSpeed`) (`self.WeightFactor`))))
    (bind _output_get_4 (set `self.FlyingVelocity` (* _output_get_2 _output_get_3)))
    (if (`self.InAirflow`)
      (set `self.AirflowSpeed` (`KismetMathLibrary.FClamp` (+ _airflowspeed_2 (* (`self.AirflowAcceleration`) _returnvalue_3)) 0.0 (`self.AirflowIntensity`)))
      (`SceneComponent.K2_SetWorldLocation` _sceneroot_2 (+ (`SceneComponent.K2_GetComponentLocation` _sceneroot_2) (* (+ _output_get_4 (* (0.0 0.0 1.0) _airflowspeed_2)) _returnvalue_3)) false false)
      (else
        (if (> _flyingdirection_z 0.001)
          (set `self.FlyingDirection` (`KismetMathLibrary.MakeVector` _flyingdirection_x _flyingdirection_y)))
        (bind _output_get_5 (set `self.VerticalAcceleration` (+ (* (`self.G`) -1.0) (* (`self.AirDrag`) (`KismetMathLibrary.DegCos` _returnvalue_7)))))
        (set `self.VerticalSpeed` (+ (`self.VerticalSpeed`) (* _output_get_5 _returnvalue_3)))
        (if (> _airflowspeed 0.01)
          (set `self.AirflowSpeed` (- _airflowspeed (* (`self.AirflowFadeOutAcceleration`) _returnvalue_3)))
          (`SceneComponent.K2_SetWorldLocation` _sceneroot_3 (+ _returnvalue_6 (+ (* (`self.FlyingVelocity`) _returnvalue_2) (`KismetMathLibrary.MakeVector` 0.0 0.0 _returnvalue_8) (* (* (0.0 0.0 1.0) (`self.AirflowSpeed`)) _returnvalue_2))) false false)
          (else
            (`SceneComponent.K2_SetWorldLocation` _sceneroot_3 (+ _returnvalue_6 (+ (* (`self.FlyingVelocity`) _returnvalue_2) (`KismetMathLibrary.MakeVector` 0.0 0.0 _returnvalue_8))) false false)))))
    (bind _output_get_6 (set `self.TotalTurningDegree` (+ (`self.TargetMeshLocalRotationX`) (`self.TargetMeshLocalRotationZ`))))
    (`SceneComponent.K2_SetWorldRotation` _sceneroot (`KismetMathLibrary.MakeRotator` 0.0 0.0 (+ _returnvalue_yaw (* (`self.TurningSpeed`) (`KismetMathLibrary.FClamp` (/ _output_get_6 180.0) -1.0) _returnvalue_2))) false false)))

(fn `Land`
  (set `self.InAir` false))

(fn `StopYawInput`
  (set `self.TargetMeshLocalRotationZ` 0.0))

(fn `TakeOff`
  (params (TakeOffSpeed :type "Float (double-precision)"))
  (set `self.OriginalFlyingSpeed` TakeOffSpeed)
  (set `self.CurrentFlyingSpeed` TakeOffSpeed)
  (set `self.InAir` true))
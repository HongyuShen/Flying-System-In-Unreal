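; Aircraft flight component that moves and turns its owning pawn, with takeoff gated by ground speed and separate airborne and ground-contact states.
; Yaw, pitch and roll inputs set clamped target angles that the mesh root lerps toward each tick.
; In air, the pawn moves along mesh forward at boostable speed, scaled by optional power and weight curves.
; Roll plus yaw turns the pawn; pitch input toggles collision sweep by height.
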(event `self.ReceiveTick`
  (params (DeltaSeconds :type "Float (single-precision)"))
  (if (`self.EnabledFlyingLogic`)
    (`self.Fly`)))

(fn `AddPitchInput`
  (params (Value :type "Float (double-precision)"))
  (bind (_returnvalue_x _returnvalue_y _returnvalue_z) (`KismetMathLibrary.BreakVector` (`Actor.K2_GetActorLocation` (`self.Pawn`))))
  (set `self.TargetMeshLocalRotationY` (`KismetMathLibrary.FClamp` (+ (`self.TargetMeshLocalRotationY`) (* Value (`self.MeshPitchTurningSpeed`) (`GameplayStatics.GetWorldDeltaSeconds`))) -89.995003 89.995003))
  (if (> (- _returnvalue_z (`self.CurrentGroundHeight`)) (`self.MinimumSweepHeight`))
    (set `self.EnabledSweep` true)
    (else
      (set `self.EnabledSweep` false))))

(fn `AddRollInput`
  (params (Value :type "Float (double-precision)"))
  (if (not (`self.TouchedGround`))
    (set `self.TargetMeshLocalRotationX` (`KismetMathLibrary.FClamp` (+ (`self.TargetMeshLocalRotationX`) (* Value (`self.MeshRollTurningSpeed`) (`GameplayStatics.GetWorldDeltaSeconds`))) -179.899994 179.899994))))

(fn `AddWeight`
  (params (IncreaseValue :type "Float (double-precision)"))
  (bind _maximumcarryingweight (`self.MaximumCarryingWeight`))
  (set `self.CurrentCarryingWeight` (`KismetMathLibrary.FClamp` (+ (`self.CurrentCarryingWeight`) IncreaseValue) 0.0 _maximumcarryingweight))
  (set `self.WeightPercentage` (/ (`self.WeightPercentage`) _maximumcarryingweight)))

(fn `AddYawInput`
  (params (Value :type "Float (double-precision)"))
  (bind _maximummeshyawangle (`self.MaximumMeshYawAngle`))
  (if (not (`self.TouchedGround`))
    (set `self.TargetMeshLocalRotationZ` (`KismetMathLibrary.FClamp` (+ (`self.TargetMeshLocalRotationZ`) (* Value (`self.MeshYawTurningSpeed`) (`GameplayStatics.GetWorldDeltaSeconds`))) (* _maximummeshyawangle -1.0) _maximummeshyawangle))))

(fn `Fly`
  (bind _returnvalue (`GameplayStatics.GetWorldDeltaSeconds`))
  (bind _returnvalue_2 (`GameplayStatics.GetWorldDeltaSeconds`))
  (bind _meshroot (`self.MeshRoot`))
  (bind _pawn (`self.Pawn`))
  (bind _pawn_2 (`self.Pawn`))
  (bind _currentflyingspeed (`self.CurrentFlyingSpeed`))
  (bind _normalflyingspeed (`self.NormalFlyingSpeed`))
  (bind (_returnvalue_roll _returnvalue_pitch _returnvalue_yaw) (`KismetMathLibrary.BreakRotator` (`Actor.K2_GetActorRotation` _pawn)))
  (bind (_returnvalue_x _returnvalue_y _returnvalue_z) (`KismetMathLibrary.BreakVector` (`Actor.K2_GetActorLocation` (`self.Pawn`))))
  (bind _returnvalue_3 (* (`self.BoostAcceleration`) (`GameplayStatics.GetWorldDeltaSeconds`)))
  (bind (_relativerotation_roll _relativerotation_pitch _relativerotation_yaw) (`KismetMathLibrary.BreakRotator` (`SceneComponent.RelativeRotation` _meshroot)))
  (bind _returnvalue_4 (`KismetMathLibrary.Lerp` _relativerotation_roll (`self.TargetMeshLocalRotationX`) (* (`self.MeshRollTurningSmoothingFactor`) _returnvalue)))
  (bind _returnvalue_5 (`KismetMathLibrary.Lerp` _relativerotation_pitch (`self.TargetMeshLocalRotationY`) (* (`self.MeshPitchTurningSmoothingFactor`) _returnvalue)))
  (bind _returnvalue_6 (+ (`self.CurrentFlyingSpeed`) _returnvalue_3))
  (if (`self.TouchedGround`)
    (set `self.CurrentGroundHeight` _returnvalue_z)
    ;[1 1 1] Reset Roll And Pich To 0
    (`SceneComponent.K2_SetRelativeRotation` (`self.MeshRoot`) (`KismetMathLibrary.MakeRotator` _returnvalue_4 _returnvalue_5 _relativerotation_yaw) false false)
    (else
      ;[1 1 1] Rotation
      (`SceneComponent.K2_SetRelativeRotation` _meshroot (`KismetMathLibrary.MakeRotator` _returnvalue_4 _returnvalue_5 (`KismetMathLibrary.Lerp` _relativerotation_yaw (`self.TargetMeshLocalRotationZ`) (* (`self.MeshYawTurningSmoothingFactor`) _returnvalue))) false false)))
  (if (`self.InAir`)
    ;[1 1 1] Power Consumption
    (if (`self.CalculatePowerConsumption`)
      (if (`self.Boosting`)
        (set `self.CurrentPower` (`KismetMathLibrary.FClamp` (- (`self.CurrentPower`) (* (`self.PowerDecreaseSpeed`) (`GameplayStatics.GetWorldDeltaSeconds`))) 0.0 (`self.MaximumPower`)))
        (else
          (set `self.CurrentPower` (`KismetMathLibrary.FClamp` (- (`self.CurrentPower`) (* (`self.PowerDecreaseSpeedWhenBoosting`) (`GameplayStatics.GetWorldDeltaSeconds`))) 0.0 (`self.MaximumPower`)))))
      (bind _output_get (set `self.PowerPercentage` (/ (`self.CurrentPower`) (`self.MaximumPower`))))
      (set `self.PowerFactor` (`CurveFloat.GetFloatValue` (`self.SpeedRemainingPowerRatioCurve`) (- 1.0 _output_get)))
      (else
        (set `self.PowerFactor` 1.0)))
    ;[1 1 1] Carrying Weight
    (if (`self.CalculateCarryingWeight`)
      (bind _output_get_2 (set `self.WeightPercentage` (/ (`self.CurrentCarryingWeight`) (`self.MaximumCarryingWeight`))))
      (set `self.WeightFactor` (`CurveFloat.GetFloatValue` (`self.SpeedCarryingWeightRatioCurve`) _output_get_2))
      (else
        (set `self.WeightFactor` 1.0)))
    ;[1 1 1] Displacement
    (if (`self.Boosting`)
      (set `self.CurrentFlyingSpeed` (`KismetMathLibrary.FClamp` _returnvalue_6 0.0 (`self.MaximumFlyingSpeed`)))
      (elif (> _currentflyingspeed _normalflyingspeed)
        (set `self.CurrentFlyingSpeed` (- _currentflyingspeed _returnvalue_3))
        (else
          (set `self.CurrentFlyingSpeed` (`KismetMathLibrary.FClamp` _returnvalue_6 0.0 _normalflyingspeed)))))
    (bind _output_get_3 (set `self.FlyingDirection` (`SceneComponent.GetForwardVector` (`self.MeshRoot`))))
    (bind _output_get_4 (set `self.FlyingSpeed` (* (`self.CurrentFlyingSpeed`) (`self.PowerFactor`) (`self.WeightFactor`))))
    (bind _output_get_5 (set `self.FlyingVelocity` (* _output_get_3 _output_get_4)))
    (`Actor.K2_SetActorLocation` _pawn_2 (+ (`Actor.K2_GetActorLocation` _pawn_2) (* _output_get_5 _returnvalue_2)) (`self.EnabledSweep`) false)
    ;[1 1 1] Turning
    (bind _output_get_6 (set `self.TotalTurningDegree` (+ (`self.TargetMeshLocalRotationX`) (`self.TargetMeshLocalRotationZ`))))
    (`Actor.K2_SetActorRotation` _pawn (`KismetMathLibrary.MakeRotator` 0.0 0.0 (+ _returnvalue_yaw (* (`self.TurningSpeed`) (`KismetMathLibrary.FClamp` (/ _output_get_6 180.0) -1.0) _returnvalue_2))) false)))

(fn `Land`
  (set `self.InAir` false))

(fn `LeaveGround`
  (set `self.TouchedGround` false))

(fn `StopYawInput`
  (set `self.TargetMeshLocalRotationZ` 0.0))

(fn `TakeOff`
  (params (GroundMovementSpeed :type "Float (double-precision)"))
  (returns (Result :type Boolean))
  (if (> GroundMovementSpeed (`self.MinimumTakeOffSpeed`))
    (set `self.CurrentFlyingSpeed` (`self.NormalFlyingSpeed`))
    (set `self.InAir` true))
  (return (`self.InAir`)))

(fn `TouchGround`
  (if (not (`self.InAir`))
    (set `self.TouchedGround` true)
    (set `self.TargetMeshLocalRotationX` 0.0)
    (set `self.TargetMeshLocalRotationY` 0.0)))
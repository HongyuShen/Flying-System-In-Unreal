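; Creature flying component that drives flight, from takeoff to landing, by moving the scene root without sweep each tick.
; Yaw input takes the flight direction from the camera, and the mesh eases toward it with banked roll and wrap-safe yaw interpolation.
; Fly integrates boost, slowdown and gravity-driven dive speeds, scaled by stamina and carried-weight curves.
; Airflow forces feed a vertical velocity term and pause stamina drain and diving.
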(event `self.ReceiveTick`
  (params (DeltaSeconds :type "Float (single-precision)"))
  (if (`self.EnabledFlyingLogic`)
    (`self.Fly`)))

(fn `AddAirflowForce`
  (params (Intensity :type "Float (double-precision)") (Acceleration :type "Float (double-precision)") (FadeOutAcceleration :type "Float (double-precision)"))
  (set `self.AirflowIntensity` Intensity)
  (set `self.AirflowAcceleration` Acceleration)
  (set `self.AirflowFadeOutAcceleration` FadeOutAcceleration)
  (set `self.InAirflow` true))

(fn `AddWeight`
  (params (IncreaseValue :type "Float (double-precision)"))
  (bind _maximumcarryingweight (`self.MaximumCarryingWeight`))
  (set `self.CurrentCarryingWeight` (`KismetMathLibrary.FClamp` (+ (`self.CurrentCarryingWeight`) IncreaseValue) 0.0 _maximumcarryingweight))
  (set `self.WeightPercentage` (/ (`self.WeightPercentage`) _maximumcarryingweight)))

(fn `AddYawInput`
  (params (Value :type "Float (double-precision)"))
  (bind (_targetmeshlocalrotation_roll _targetmeshlocalrotation_pitch _targetmeshlocalrotation_yaw) (`KismetMathLibrary.BreakRotator` (`self.TargetMeshLocalRotation`)))
  (bind (_returnvalue_x _returnvalue_y _returnvalue_z) (`KismetMathLibrary.BreakVector` (`SceneComponent.K2_GetComponentLocation` (`self.SceneRoot`))))
  (bind (_relativerotation_roll _relativerotation_pitch _relativerotation_yaw) (`KismetMathLibrary.BreakRotator` (`SceneComponent.RelativeRotation` (`self.MeshRoot`))))
  (bind _returnvalue (- _targetmeshlocalrotation_yaw _relativerotation_yaw))
  (if (> (`KismetMathLibrary.Abs` Value) 0.025)
    (bind _output_get (set `self.FlyingDirection` (`KismetMathLibrary.Normal` (- (`KismetMathLibrary.MakeVector` _returnvalue_x _returnvalue_y (+ _returnvalue_z (`self.CameraLookAtMeshOffsetZ`))) (`SceneComponent.K2_GetComponentLocation` (`self.Camera`))))))
    (set `self.TargetMeshLocalRotation` (`KismetMathLibrary.FindLookAtRotation` (0.0 0.0 0.0) _output_get))
    (set `self.RelativeRotationZ` 0.0)
    (set `self.RotationZAlignmentPercentage` 0.0)
    (if (> _returnvalue 180.0)
      (set `self.DeltaRotationZ` (- 360.0 _returnvalue))
      (else
        (set `self.DeltaRotationZ` _returnvalue)))
    (if (> (`self.DeltaRotationZ`) 10.0)
      (set `self.AlignedToTargetDirection` false))
    (if (< Value 0.0)
      (set `self.TurningDirection` 1.0)
      (else
        (set `self.TurningDirection` -1.0)))))

(fn `ConvertTo360Degree`
  (params (Angle :type "Float (double-precision)"))
  (returns (ResultAngle :type "Float (double-precision)"))
  (if (< Angle 0.0)
    (return (+ 360.0 Angle))
    (else
      (return Angle))))

(fn `EndAirflowForce`
  (set `self.InAirflow` false))

(fn `Fly`
  (bind _returnvalue (`GameplayStatics.GetWorldDeltaSeconds`))
  (bind _returnvalue_2 (`GameplayStatics.GetWorldDeltaSeconds`))
  (bind _returnvalue_3 (`GameplayStatics.GetWorldDeltaSeconds`))
  (bind _returnvalue_4 (`GameplayStatics.GetWorldDeltaSeconds`))
  (bind _airflowspeed (`self.AirflowSpeed`))
  (bind _flyingvelocity (`self.FlyingVelocity`))
  (bind (_targetmeshlocalrotation_roll _targetmeshlocalrotation_pitch) (`KismetMathLibrary.BreakRotator` (`self.TargetMeshLocalRotation`)))
  (bind (_targetmeshlocalrotation_roll_2 _targetmeshlocalrotation_pitch_2 _targetmeshlocalrotation_yaw) (`KismetMathLibrary.BreakRotator` (`self.TargetMeshLocalRotation`)))
  (bind _meshroot (`self.MeshRoot`))
  (bind _verticalspeed (`self.VerticalSpeed`))
  (bind _currentflyingspeed (`self.CurrentFlyingSpeed`))
  (bind _currentflyingspeed_2 (`self.CurrentFlyingSpeed`))
  (bind _decelerationafterdiving (`self.DecelerationAfterDiving`))
  (bind _currentflyingspeed_3 (`self.CurrentFlyingSpeed`))
  (bind _returnvalue_5 (`SceneComponent.K2_GetComponentLocation` (`self.SceneRoot`)))
  (bind _returnvalue_6 (> _currentflyingspeed_2 (`self.NormalFlyingSpeed`)))
  (bind _returnvalue_7 (> _currentflyingspeed_3 (`self.MaximumFlyingSpeed`)))
  (bind (_relativerotation_roll _relativerotation_pitch _relativerotation_yaw) (`KismetMathLibrary.BreakRotator` (`SceneComponent.RelativeRotation` (`self.MeshRoot`))))
  (bind (_relativerotation_roll_2 _relativerotation_pitch_2) (`KismetMathLibrary.BreakRotator` (`SceneComponent.RelativeRotation` (`self.MeshRoot`))))
  (bind (_relativerotation_roll_3 _relativerotation_pitch_3) (`KismetMathLibrary.BreakRotator` (`SceneComponent.RelativeRotation` _meshroot)))
  (bind (_relativerotation_roll_4 _relativerotation_pitch_4) (`KismetMathLibrary.BreakRotator` (`SceneComponent.RelativeRotation` (`self.MeshRoot`))))
  (bind (_relativerotation_roll_5 _relativerotation_pitch_5) (`KismetMathLibrary.BreakRotator` (`SceneComponent.RelativeRotation` (`self.MeshRoot`))))
  (bind _returnvalue_8 (`KismetMathLibrary.InRange_FloatFloat` _relativerotation_pitch_2 0.0 89.995003 false false))
  (bind _returnvalue_9 (- _currentflyingspeed_3 (* _decelerationafterdiving _returnvalue_2)))
  (bind _returnvalue_10 (+ _currentflyingspeed_3 (* (`self.BoostAcceleration`) _returnvalue_2)))
  (bind _returnvalue_11 (`KismetMathLibrary.FClamp` _returnvalue_10 0.0 (`self.MaximumFlyingSpeed`)))
  (bind _returnvalue_12 (`KismetMathLibrary.DegCos` (+ _relativerotation_pitch_5 90.0)))
  (bind _returnvalue_13 (`KismetMathLibrary.FClamp` _returnvalue_10 0.0 (`self.NormalFlyingSpeed`)))
  (bind _returnvalue_14 (+ _returnvalue_5 (* (+ _flyingvelocity (`KismetMathLibrary.MakeVector` 0.0 0.0 (`self.AirflowSpeed`))) _returnvalue)))
  (bind _returnvalue_15 (- _currentflyingspeed_3 (+ (`self.DecelerationAfterDiving`) (* _decelerationafterdiving (`KismetMathLibrary.DegSin` _relativerotation_pitch_2) _returnvalue_2))))
  (if (`self.InAir`)
    (if (not (`self.SlowingDown`))
      (bind _output_get (set `self.RotationZComponent` (* (`self.MeshHorizontalTurningSpeed`) (`GameplayStatics.GetWorldDeltaSeconds`))))
      (set `self.CurrentMeshLocalRotationZ` (`self.RotationLerp` (`self.ConvertTo360Degree` _relativerotation_yaw) (`self.ConvertTo360Degree` _targetmeshlocalrotation_yaw) _output_get))
      (if (not (`self.AlignedToTargetDirection`))
        (bind _output_get_2 (set `self.RelativeRotationZ` (+ (`self.RelativeRotationZ`) (`self.IncreaseAngle`))))
        (bind _output_get_3 (set `self.RotationZAlignmentPercentage` (`KismetMathLibrary.FClamp` (/ _output_get_2 (`self.DeltaRotationZ`)))))
        (if (> _output_get_3 0.985)
          (set `self.AlignedToTargetDirection` true))
        (set `self.TargetMeshLocalRotationX` (`KismetMathLibrary.Lerp` _relativerotation_roll_3 (* (`self.TurningDirection`) (`self.MeshMaximumTurningRotationX`)) (* (`self.RotationZAlignmentPercentage`) (`self.MeshRotationXSmoothingFactor`))))
        (else
          (set `self.TargetMeshLocalRotationX` (`KismetMathLibrary.Lerp` _relativerotation_roll_3 0.0 (`self.RotationZComponent`)))))
      (`SceneComponent.K2_SetRelativeRotation` _meshroot (`KismetMathLibrary.MakeRotator` (`self.TargetMeshLocalRotationX`) (`KismetMathLibrary.Lerp` _relativerotation_pitch_3 _targetmeshlocalrotation_pitch (* (`self.MeshVerticalTurningSpeed`) (`GameplayStatics.GetWorldDeltaSeconds`))) (`self.CurrentMeshLocalRotationZ`)) false false))
    ;[1 1 1] Stamina Consumption
    (if (`self.CalculateStaminaConsumption`)
      (if (not (`self.InAirflow`))
        (if (`self.Boosting`)
          (set `self.CurrentStamina` (`KismetMathLibrary.FClamp` (- (`self.CurrentStamina`) (* (`self.StaminaDecreaseSpeed`) (`GameplayStatics.GetWorldDeltaSeconds`))) 0.0 (`self.MaximumStamina`)))
          (else
            (set `self.CurrentStamina` (`KismetMathLibrary.FClamp` (- (`self.CurrentStamina`) (* (`self.StaminaDecreaseSpeedWhenBoosting`) (`GameplayStatics.GetWorldDeltaSeconds`))) 0.0 (`self.MaximumStamina`)))))
        (bind _output_get_4 (set `self.StaminaPercentage` (/ (`self.CurrentStamina`) (`self.MaximumStamina`))))
        (set `self.StaminaFactor` (`CurveFloat.GetFloatValue` (`self.SpeedRemainingPowerRatioCurve`) (- 1.0 _output_get_4))))
      (else
        (set `self.StaminaFactor` 1.0)))
    ;[1 1 1] Carrying Weight
    (if (`self.CalculateCarryingWeight`)
      (bind _output_get_5 (set `self.WeightPercentage` (/ (`self.CurrentCarryingWeight`) (`self.MaximumCarryingWeight`))))
      (set `self.WeightFactor` (`CurveFloat.GetFloatValue` (`self.SpeedCarryingWeightRatioCurve`) _output_get_5))
      (else
        (set `self.WeightFactor` 1.0)))
    (if (and (not (`self.InAirflow`)) (`self.CanDive`) (> _relativerotation_pitch_4 -89.995003) (< _relativerotation_pitch_4 (* (`self.DivingStartAngle`) -1.0)))
      (set `self.Diving` true)
      (if (`self.SlowingDown`)
        (set `self.CurrentFlyingSpeed` (`KismetMathLibrary.FClamp` (- _currentflyingspeed (* (`self.SlowDownAcceleration`) _returnvalue_4)) 0.0 _currentflyingspeed))
        (set `self.VerticalAcceleration` (- (`self.SlowDownAcceleration`) (* (`self.G`) _returnvalue_12)))
        (else
          (set `self.CurrentFlyingSpeed` (`KismetMathLibrary.FClamp` (+ _currentflyingspeed (* (+ (`self.BoostAcceleration`) (* (`self.G`) (`KismetMathLibrary.DegSin` (* _relativerotation_pitch_5 -1.0)))) _returnvalue_4)) 0.0 (`self.MaximumDivingSpeed`)))
          (set `self.VerticalAcceleration` (* (`self.G`) -1.0 _returnvalue_12))))
      (bind _output_get_6 (set `self.FlyingSpeed` (* (`self.CurrentFlyingSpeed`) (`self.StaminaFactor`) (`self.WeightFactor`))))
      (set `self.FlyingVelocity` (* (`self.FlyingDirection`) _output_get_6))
      (set `self.VerticalSpeed` (+ (`self.VerticalSpeed`) (* (`self.VerticalAcceleration`) _returnvalue_3)))
      (set `self.TargetCharacterLocation` (+ (`SceneComponent.K2_GetComponentLocation` (`self.SceneRoot`)) (* (`self.FlyingVelocity`) _returnvalue_3) (`KismetMathLibrary.MakeVector` 0.0 0.0 (`KismetMathLibrary.FClamp` (- (* (`self.VerticalSpeed`) _returnvalue_3) (* 0.5 (`self.VerticalAcceleration`) _returnvalue_3 _returnvalue_3)) 0.0 -100000000.0))))
      (elif (not (`self.StopFlying`))
        (set `self.Diving` false)
        (if (< _verticalspeed -0.1)
          (set `self.VerticalSpeed` (+ _verticalspeed (* (`self.AirDrag`) (`KismetMathLibrary.DegCos` (* _relativerotation_pitch_5 -1.0)) (`GameplayStatics.GetWorldDeltaSeconds`))))
          (else
            (set `self.VerticalSpeed` 0.0)))
        (if (`self.Boosting`)
          (if _returnvalue_8
            (if _returnvalue_7
              (set `self.CurrentFlyingSpeed` _returnvalue_15)
              (else
                (set `self.CurrentFlyingSpeed` _returnvalue_11)))
            (elif _returnvalue_7
              (set `self.CurrentFlyingSpeed` _returnvalue_9)
              (else
                (set `self.CurrentFlyingSpeed` _returnvalue_11))))
          (elif (`self.SlowingDown`)
            (if _returnvalue_8
              (if _returnvalue_6
                (set `self.CurrentFlyingSpeed` _returnvalue_15))
              (elif _returnvalue_6
                (set `self.CurrentFlyingSpeed` _returnvalue_9)))
            (set `self.CurrentFlyingSpeed` (`KismetMathLibrary.FClamp` (- _currentflyingspeed_2 (* (`self.SlowDownAcceleration`) (`GameplayStatics.GetWorldDeltaSeconds`))) 0.0 _currentflyingspeed_2))
            (elif _returnvalue_8
              (if _returnvalue_6
                (set `self.CurrentFlyingSpeed` _returnvalue_15)
                (else
                  (set `self.CurrentFlyingSpeed` _returnvalue_13)))
              (elif _returnvalue_6
                (set `self.CurrentFlyingSpeed` _returnvalue_9)
                (else
                  (set `self.CurrentFlyingSpeed` _returnvalue_13))))))
        (bind _output_get_7 (set `self.FlyingSpeed` (* (`self.CurrentFlyingSpeed`) (`self.StaminaFactor`) (`self.WeightFactor`))))
        (set `self.FlyingVelocity` (* (`self.FlyingDirection`) _output_get_7))
        (if (> _airflowspeed 0.01)
          (set `self.AirflowSpeed` (- _airflowspeed (* (`self.AirflowFadeOutAcceleration`) _returnvalue)))
          (set `self.TargetCharacterLocation` _returnvalue_14)
          (else
            (set `self.TargetCharacterLocation` (+ _returnvalue_5 (* _flyingvelocity _returnvalue)))))
        (else
          (set `self.StaminaRecoverySpeed` (`KismetMathLibrary.FClamp` (+ (`self.CurrentStamina`) (* (`self.StaminaRecoverySpeed`) (`GameplayStatics.GetWorldDeltaSeconds`))) 0.0 (`self.MaximumStamina`)))
          (bind _output_get_8 (set `self.FlyingSpeed` (`self.CurrentFlyingSpeed`)))
          (set `self.FlyingVelocity` (* (`self.FlyingDirection`) _output_get_8))
          (if (`self.InAirflow`)
            (set `self.AirflowSpeed` (`KismetMathLibrary.FClamp` (+ (`self.AirflowSpeed`) (* (`self.AirflowAcceleration`) (`GameplayStatics.GetWorldDeltaSeconds`))) 0.0 (`self.AirflowIntensity`)))
            (set `self.TargetCharacterLocation` _returnvalue_14)))))
    (`SceneComponent.K2_SetWorldLocation` (`self.SceneRoot`) (`self.TargetCharacterLocation`) false false)
    (else
      (set `self.StaminaRecoverySpeed` (`KismetMathLibrary.FClamp` (+ (`self.CurrentStamina`) (* (`self.StaminaRecoverySpeed`) (`GameplayStatics.GetWorldDeltaSeconds`))) 0.0 (`self.MaximumStamina`))))))

(fn `FlyForward`
  (set `self.SlowingDown` false))

(fn `Land`
  (bind _meshroot (`self.MeshRoot`))
  (bind (_relativerotation_roll _relativerotation_pitch _relativerotation_yaw) (`KismetMathLibrary.BreakRotator` (`SceneComponent.RelativeRotation` _meshroot)))
  (set `self.InAir` false)
  (set `self.StopFlying` true)
  (if (`self.ResetMeshRotationAfterLanding`)
    (`SceneComponent.K2_SetRelativeRotation` _meshroot (`KismetMathLibrary.MakeRotator` 0.0 0.0 _relativerotation_yaw) false false)))

(fn `RotationLerp`
  (params (Angle :type "Float (double-precision)") (TargetAngle :type "Float (double-precision)") (Alpha :type "Float (double-precision)"))
  (returns (ResultAngle :type "Float (double-precision)"))
  (if (and (> Angle 270.0) (< TargetAngle 90.0))
    (bind _output_get (set `self.IncreaseAngle` (* (+ (- 360.0 Angle) TargetAngle) Alpha)))
    (return (mod (+ Angle _output_get) 360.0))
    (elif (and (< Angle 90.0) (> TargetAngle 270.0))
      (bind _output_get_2 (set `self.IncreaseAngle` (* (+ (- 360.0 TargetAngle) Angle) Alpha)))
      (return (mod (+ TargetAngle _output_get_2) 360.0))
      (else
        (bind _output_get_3 (set `self.IncreaseAngle` (- TargetAngle Angle)))
        (if (and (> TargetAngle Angle) (< _output_get_3 180.0))
          (return (+ Angle (* _output_get_3 Alpha)))
          (else
            (bind _output_get_4 (set `self.IncreaseAngle` (- Angle TargetAngle)))
            (return (- Angle (* _output_get_4 Alpha)))))))))

(fn `SlowDown`
  (set `self.Boosting` false)
  (set `self.SlowingDown` true))

(fn `StopSlowingDown`
  (set `self.SlowingDown` false))

(fn `TakeOff`
  (set `self.FlyingDirection` (`SceneComponent.GetForwardVector` (`self.MeshRoot`)))
  (`SceneComponent.K2_SetRelativeRotation` :`self` (`self.MeshRoot`))
  (set `self.CurrentFlyingSpeed` (`self.NormalFlyingSpeed`))
  (set `self.StopFlying` false)
  (set `self.InAir` true))
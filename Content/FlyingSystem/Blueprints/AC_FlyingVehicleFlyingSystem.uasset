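; Flying vehicle component that steers a mesh root and moves a scene root while airborne.
; Input functions set target yaw, pitch and roll, which Fly interpolates each tick, with optional pitch leveling when hovering.
; Speed accelerates, boosts or slows, then is scaled by optional curve-driven power and carried-weight factors.
; The resulting velocity follows the mesh's forward vector and is applied by setting world location without sweep, so no collision blocks it.
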(event `self.ReceiveTick`
  (params (DeltaSeconds :type "Float (single-precision)"))
  (if (`self.EnabledFlyingLogic`)
    (`self.Fly`)))

(fn `AddForwardInput`
  (params (Value :type "Float (double-precision)"))
  (set `self.IsMovingForward` true)
  (set `self.ForwardDirection` Value))

(fn `AddPitchInput`
  (params (Value :type "Float (double-precision)"))
  (set `self.IsLookingUp` true)
  (set `self.TargetMeshLocalRotationY` (+ (`self.TargetMeshLocalRotationY`) (* Value (`self.MeshPitchTurningSpeed`) (`GameplayStatics.GetWorldDeltaSeconds`)))))

(fn `AddWeight`
  (params (IncreaseValue :type "Float (double-precision)"))
  (bind _maximumcarryingweight (`self.MaximumCarryingWeight`))
  (set `self.CurrentCarryingWeight` (`KismetMathLibrary.FClamp` (+ (`self.CurrentCarryingWeight`) IncreaseValue) 0.0 _maximumcarryingweight))
  (set `self.WeightPercentage` (/ (`self.WeightPercentage`) _maximumcarryingweight)))

(fn `AddYawInput`
  (params (Value :type "Float (double-precision)"))
  (bind _targetmeshlocalrotationz (`self.TargetMeshLocalRotationZ`))
  (bind _returnvalue (* Value (`self.MeshYawTurningSpeed`) (`GameplayStatics.GetWorldDeltaSeconds`)))
  (bind _returnvalue_2 (+ _targetmeshlocalrotationz _returnvalue))
  (set `self.IsTurning` true)
  (if (`self.IsMovingForward`)
    (if (> (`self.ForwardDirection`) 0.0)
      (set `self.TargetMeshLocalRotationZ` _returnvalue_2)
      (else
        (set `self.TargetMeshLocalRotationZ` (- _targetmeshlocalrotationz _returnvalue))))
    (else
      (set `self.TargetMeshLocalRotationZ` _returnvalue_2)))
  (set `self.TargetMeshLocalRotationX` (* Value 1.0 (`self.MaximumMeshRollAngle`))))

(fn `Fly`
  (bind _returnvalue (`GameplayStatics.GetWorldDeltaSeconds`))
  (bind _returnvalue_2 (`GameplayStatics.GetWorldDeltaSeconds`))
  (bind _meshroot (`self.MeshRoot`))
  (bind _meshroot_2 (`self.MeshRoot`))
  (bind _sceneroot (`self.SceneRoot`))
  (bind _forwarddirection (`self.ForwardDirection`))
  (bind _maximumforwardspeed (`self.MaximumForwardSpeed`))
  (bind _normalforwardspeed (`self.NormalForwardSpeed`))
  (bind _currentflyingspeed (`self.CurrentFlyingSpeed`))
  (bind _currentflyingspeed_2 (`self.CurrentFlyingSpeed`))
  (bind _returnvalue_3 (* (`self.BoostAcceleration`) _returnvalue_2))
  (bind _returnvalue_4 (* (`self.MeshRollTurningSmoothingFactor`) _returnvalue))
  (bind _returnvalue_5 (* (`self.BackwardSpeed`) -1.0))
  (bind _returnvalue_6 (* (`self.SlowDownAcceleration`) _returnvalue_2))
  (bind (_relativerotation_roll _relativerotation_pitch _relativerotation_yaw) (`KismetMathLibrary.BreakRotator` (`SceneComponent.RelativeRotation` _meshroot)))
  (bind (_relativerotation_roll_2 _relativerotation_pitch_2 _relativerotation_yaw_2) (`KismetMathLibrary.BreakRotator` (`SceneComponent.RelativeRotation` _meshroot_2)))
  (bind _returnvalue_7 (- _currentflyingspeed _returnvalue_3))
  (bind (_returnvalue_roll _returnvalue_pitch _returnvalue_yaw) (`KismetMathLibrary.BreakRotator` (`KismetMathLibrary.RLerp` (`KismetMathLibrary.MakeRotator` 0.0 0.0 _relativerotation_yaw_2) (`KismetMathLibrary.MakeRotator` 0.0 0.0 (`self.TargetMeshLocalRotationZ`)) (* (`self.MeshYawTurningSmoothingFactor`) _returnvalue) true)))
  (bind _returnvalue_8 (+ (`self.CurrentFlyingSpeed`) _returnvalue_3))
  (if (`self.InAir`)
    (`SceneComponent.K2_SetRelativeRotation` _meshroot_2 (`KismetMathLibrary.MakeRotator` _relativerotation_roll_2 _relativerotation_pitch_2 _returnvalue_yaw) false false)
    (if (`self.IsTurning`)
      (`SceneComponent.K2_SetRelativeRotation` _meshroot_2 (`KismetMathLibrary.MakeRotator` (`KismetMathLibrary.Lerp` _relativerotation_roll_2 (`self.TargetMeshLocalRotationX`) _returnvalue_4) _relativerotation_pitch_2 _relativerotation_yaw_2) false false)
      (else
        (`SceneComponent.K2_SetRelativeRotation` _meshroot_2 (`KismetMathLibrary.MakeRotator` (`KismetMathLibrary.Lerp` _relativerotation_roll_2 0.0 _returnvalue_4) _relativerotation_pitch_2 _relativerotation_yaw_2) false false)))
    (if (and (not (`self.IsMovingForward`)) (not (`self.IsTurning`)) (not (`self.IsLookingUp`)) (`self.RemainPitchZeroWhenHovering`))
      (set `self.TargetMeshLocalRotationY` (`KismetMathLibrary.Lerp` (`self.TargetMeshLocalRotationY`) 0.0 (* (`self.MeshPitchTurningRecoverySmoothingFactor`) (`GameplayStatics.GetWorldDeltaSeconds`)))))
    (`SceneComponent.K2_SetRelativeRotation` _meshroot (`KismetMathLibrary.MakeRotator` _relativerotation_roll (`KismetMathLibrary.Lerp` _relativerotation_pitch (`self.TargetMeshLocalRotationY`) (* (`self.MeshPitchTurningSmoothingFactor`) (`GameplayStatics.GetWorldDeltaSeconds`))) _relativerotation_yaw) false false)
    ;[1 1 1] Power Consumption
    (if (`self.CalculatePowerConsumption`)
      (if (`self.Boosting`)
        (set `self.CurrentPower` (`KismetMathLibrary.FClamp` (- (`self.CurrentPower`) (* (`self.PowerDecreaseSpeed`) (`GameplayStatics.GetWorldDeltaSeconds`))) 0.0 (`self.MaximumPower`)))
        (else
          (set `self.CurrentPower` (`KismetMathLibrary.FClamp` (- (`self.CurrentPower`) (* (`self.PowerDecreaseSpeedWhenBoosting`) (`GameplayStatics.GetWorldDeltaSeconds`))) 0.0 (`self.MaximumPower`)))))
      (bind _output_get (set `self.PowerPercentage` (/ (`self.CurrentPower`) (`self.MaximumPower`))))
      (set `self.PowerFactor` (`CurveFloat.GetFloatValue` (`self.SpeedRemainingPowerRatioCurve`) (- 1.0 _output_get)))
      (else
        (set `self.PowerFactor` 1.0)))
    ;[1 1 1] Carrying Weight
    (if (`self.CalculateCarryingWeight`)
      (bind _output_get_2 (set `self.WeightPercentage` (/ (`self.CurrentCarryingWeight`) (`self.MaximumCarryingWeight`))))
      (set `self.WeightFactor` (`CurveFloat.GetFloatValue` (`self.SpeedCarryingWeightRatioCurve`) _output_get_2))
      (else
        (set `self.WeightFactor` 1.0)))
    (if (`self.IsMovingForward`)
      (if (> _forwarddirection 0.01)
        (if (`self.Boosting`)
          (set `self.CurrentFlyingSpeed` (`KismetMathLibrary.FClamp` _returnvalue_8 _returnvalue_5 _maximumforwardspeed))
          (elif (> _currentflyingspeed _normalforwardspeed)
            (set `self.CurrentFlyingSpeed` _returnvalue_7)
            (else
              (set `self.CurrentFlyingSpeed` (`KismetMathLibrary.FClamp` _returnvalue_8 _returnvalue_5 _normalforwardspeed)))))
        (elif (< _forwarddirection -0.01)
          (set `self.CurrentFlyingSpeed` (`KismetMathLibrary.FClamp` _returnvalue_7 _returnvalue_5 _maximumforwardspeed))))
      (elif (> _currentflyingspeed_2 0.0)
        (set `self.CurrentFlyingSpeed` (`KismetMathLibrary.FClamp` (- _currentflyingspeed _returnvalue_6) 0.0 _normalforwardspeed))
        (elif (< _currentflyingspeed_2 0.0)
          (set `self.CurrentFlyingSpeed` (`KismetMathLibrary.FClamp` (+ _currentflyingspeed _returnvalue_6) _returnvalue_5 0.0)))))
    (bind _output_get_3 (set `self.FlyingDirection` (`SceneComponent.GetForwardVector` (`self.MeshRoot`))))
    (bind _output_get_4 (set `self.FlyingSpeed` (* (`self.CurrentFlyingSpeed`) (`self.PowerFactor`) (`self.WeightFactor`))))
    (bind _output_get_5 (set `self.FlyingVelocity` (* _output_get_3 _output_get_4)))
    (`SceneComponent.K2_SetWorldLocation` _sceneroot (+ (`SceneComponent.K2_GetComponentLocation` _sceneroot) (* _output_get_5 (`GameplayStatics.GetWorldDeltaSeconds`))) false false)))

(fn `Land`
  (set `self.InAir` false))

(fn `LateStopTurning`
  (set `self.IsTurning` false)
  (set `self.TargetMeshLocalRotationX` 0.0))

(fn `StopMovingForward`
  (set `self.IsMovingForward` false))

(fn `StopPitchInput`
  (set `self.IsLookingUp` false))

(fn `StopTurning`
  (if (and (not (`self.IsMovingForward`)) (not (`self.IsLookingUp`)))
    (`KismetSystemLibrary.K2_SetTimer` null "LateStopTurning" (`self.MeshTurningRecoveryDelay`))
    (else
      (`self.LateStopTurning`))))

(fn `TakeOff`
  (set `self.InAir` true))
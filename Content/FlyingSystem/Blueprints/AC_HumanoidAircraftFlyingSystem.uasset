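; Actor component that flies a humanoid-style aircraft pawn through FloatingPawnMovement, ticking Fly while flying logic is enabled.
; Yaw and pitch inputs form a direction, converted to world space through a far-offset spring-arm reference arrow and flattened unless HoverMode is on.
; Boost-adjusted speed is scaled by optional curve-driven power and carried-weight factors.
; RollRoot and MeshRoot smoothly turn toward the spring arm, bank and pitch, easing level without input.
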(event `self.ReceiveTick`
  (params (DeltaSeconds :type "Float (single-precision)"))
  (if (`self.EnabledFlyingLogic`)
    (`self.Fly`)))

(fn `AddPitchInput`
  (params (Value :type "Float (double-precision)"))
  (bind (_flyingdirection_x _flyingdirection_y _flyingdirection_z) (`KismetMathLibrary.BreakVector` (`self.FlyingDirection`)))
  (set `self.FlyingDirection` (`KismetMathLibrary.MakeVector` _flyingdirection_x (+ _flyingdirection_y Value) _flyingdirection_z)))

(fn `AddWeight`
  (params (IncreaseValue :type "Float (double-precision)"))
  (bind _maximumcarryingweight (`self.MaximumCarryingWeight`))
  (set `self.CurrentCarryingWeight` (`KismetMathLibrary.FClamp` (+ (`self.CurrentCarryingWeight`) 1.0) 0.0 _maximumcarryingweight))
  (set `self.WeightPercentage` (/ (`self.WeightPercentage`) _maximumcarryingweight)))

(fn `AddYawInput`
  (params (Value :type "Float (double-precision)"))
  (bind (_flyingdirection_x _flyingdirection_y _flyingdirection_z) (`KismetMathLibrary.BreakVector` (`self.FlyingDirection`)))
  (set `self.FlyingDirection` (`KismetMathLibrary.MakeVector` (+ _flyingdirection_x Value) _flyingdirection_y _flyingdirection_z)))

(fn `DeltaAngle`
  (params (Angle1 :type "Float (double-precision)") (Angle2 :type "Float (double-precision)"))
  (returns (Angle :type "Float (double-precision)"))
  (bind _newangle1 (`self.NewAngle1`))
  (bind _newangle2 (`self.NewAngle2`))
  (if (< Angle1 0.0)
    (set `self.NewAngle1` (+ Angle1 360.0))
    (else
      (set `self.NewAngle1` Angle1)))
  (if (< Angle2 0.0)
    (set `self.NewAngle2` (+ Angle2 360.0))
    (else
      (set `self.NewAngle2` Angle2)))
  (if (and (> _newangle1 270.0) (< _newangle2 90.0))
    (return (- (+ _newangle2 360.0) _newangle1))
    (elif (and (< _newangle1 90.0) (> _newangle2 270.0))
      (return (- (+ _newangle1 360.0) _newangle2))
      (else
        (return (`KismetMathLibrary.Abs` (- _newangle2 _newangle1)))))))

(fn `Fly`
  (bind _returnvalue (`GameplayStatics.GetWorldDeltaSeconds`))
  (bind _returnvalue_2 (`GameplayStatics.GetWorldDeltaSeconds`))
  (bind _returnvalue_3 (`GameplayStatics.GetWorldDeltaSeconds`))
  (bind (_flyingdirection_x _flyingdirection_y) (`KismetMathLibrary.BreakVector` (`self.FlyingDirection`)))
  (bind _rollroot (`self.RollRoot`))
  (bind (_flyingdirection_x_2 _flyingdirection_y_2) (`KismetMathLibrary.BreakVector` (`self.FlyingDirection`)))
  (bind (_flyingdirection_x_3 _flyingdirection_y_3) (`KismetMathLibrary.BreakVector` (`self.FlyingDirection`)))
  (bind _meshroot (`self.MeshRoot`))
  (bind _currentflyingspeed (`self.CurrentFlyingSpeed`))
  (bind _normalflyingspeed (`self.NormalFlyingSpeed`))
  (bind _rollroot_2 (`self.RollRoot`))
  (bind _maximumpower (`self.MaximumPower`))
  (bind _meshroot_2 (`self.MeshRoot`))
  (bind _currentpower (`self.CurrentPower`))
  (bind (_returnvalue_roll _returnvalue_pitch _returnvalue_yaw) (`KismetMathLibrary.BreakRotator` (`SceneComponent.K2_GetComponentRotation` (`self.SpringArm`))))
  (bind (_returnvalue_roll_2 _returnvalue_pitch_2 _returnvalue_yaw_2) (`KismetMathLibrary.BreakRotator` (`SceneComponent.K2_GetComponentRotation` _rollroot)))
  (bind (_returnvalue_roll_3 _returnvalue_pitch_3 _returnvalue_yaw_3) (`KismetMathLibrary.BreakRotator` (`SceneComponent.K2_GetComponentRotation` (`self.RollRoot`))))
  (bind _returnvalue_4 (* (`self.MaximumMeshPitchAngle`) _flyingdirection_y_2))
  (bind _returnvalue_5 (* (`self.BoostAcceleration`) (`GameplayStatics.GetWorldDeltaSeconds`)))
  (bind (_relativerotation_roll _relativerotation_pitch) (`KismetMathLibrary.BreakRotator` (`SceneComponent.RelativeRotation` _meshroot)))
  (bind (_relativerotation_roll_2 _relativerotation_pitch_2 _relativerotation_yaw) (`KismetMathLibrary.BreakRotator` (`SceneComponent.RelativeRotation` _rollroot_2)))
  (bind (_relativerotation_roll_3 _relativerotation_pitch_3) (`KismetMathLibrary.BreakRotator` (`SceneComponent.RelativeRotation` _meshroot_2)))
  ;[1 1 1] Power Consumption
  (if (`self.CalculatePowerConsumption`)
    (if (`self.InAir`)
      (if (`self.Boosting`)
        (set `self.CurrentPower` (`KismetMathLibrary.FClamp` (- _currentpower (* (`self.PowerDecreaseSpeed`) _returnvalue_2)) 0.0 _maximumpower))
        (else
          (set `self.CurrentPower` (`KismetMathLibrary.FClamp` (- _currentpower (* (`self.PowerDecreaseSpeedWhenBoosting`) _returnvalue_2)) 0.0 _maximumpower))))
      (bind _output_get (set `self.PowerPercentage` (/ (`self.CurrentPower`) _maximumpower)))
      (set `self.PowerFactor` (`CurveFloat.GetFloatValue` (`self.SpeedRemainingPowerRatioCurve`) (- 1.0 _output_get))))
    (else
      (set `self.PowerFactor` 1.0)))
  ;[1 1 1] Carrying Weight
  (if (`self.CalculateCarryingWeight`)
    (bind _output_get_2 (set `self.WeightPercentage` (/ (`self.CurrentCarryingWeight`) (`self.MaximumCarryingWeight`))))
    (set `self.WeightFactor` (`CurveFloat.GetFloatValue` (`self.SpeedCarryingWeightRatioCurve`) _output_get_2))
    (else
      (set `self.WeightFactor` 1.0)))
  ;[1 1 1] Rotation
  (if (or (> (`KismetMathLibrary.Abs` _flyingdirection_x) 0.01) (> (`KismetMathLibrary.Abs` _flyingdirection_y) 0.01))
    (bind _output_get_3 (set `self.FlyingDirection` (`KismetMathLibrary.Normal` (`self.FlyingDirection`))))
    (set `self.TargetMeshLocalRotationX` (* (`self.MaximumMeshRollAngle`) (.x _output_get_3)))
    (if (not (`self.FreezeMeshRotationY`))
      (if (< (`self.DeltaAngle` _returnvalue_yaw _returnvalue_yaw_3) 90.0)
        (set `self.TargetMeshLocalRotationY` (* _returnvalue_4 -1.0))
        (else
          (set `self.TargetMeshLocalRotationY` _returnvalue_4)))
      (else
        (set `self.TargetMeshLocalRotationY` 0.0)))
    (set `self.TargetMeshLocalRotationZ` _returnvalue_yaw)
    (`SceneComponent.K2_SetWorldRotation` _rollroot_2 (`KismetMathLibrary.RLerp` (`SceneComponent.K2_GetComponentRotation` _rollroot_2) (`SceneComponent.K2_GetComponentRotation` (`self.SpringArm`)) (* (`self.MeshYawTurningSmoothingFactor`) _returnvalue) true) false false)
    (`SceneComponent.K2_SetRelativeRotation` _rollroot_2 (`KismetMathLibrary.MakeRotator` (`KismetMathLibrary.Lerp` _relativerotation_roll_2 (`self.TargetMeshLocalRotationX`) (* (`self.MeshRollTurningSmoothingFactor`) _returnvalue)) 0.0 _relativerotation_yaw) false false)
    (`SceneComponent.K2_SetRelativeRotation` _meshroot_2 (`KismetMathLibrary.MakeRotator` 0.0 (`KismetMathLibrary.Lerp` _relativerotation_pitch_3 (`self.TargetMeshLocalRotationY`) (* (`self.MeshPitchTurningSmoothingFactor`) _returnvalue))) false false)
    (`SceneComponent.K2_SetRelativeLocation` (`self.SpringArmLocalReferenceArrow`) (`KismetMathLibrary.MakeVector` (* _flyingdirection_y_3 1000000.0) (* _flyingdirection_x_3 1000000.0)) false false)
    (if (`self.Boosting`)
      ;[1 1 1] Calculate Speed
      (set `self.CurrentFlyingSpeed` (`KismetMathLibrary.FClamp` (+ (`self.CurrentFlyingSpeed`) _returnvalue_5) 0.0 (`self.MaximumFlyingSpeed`)))
      (elif (> _currentflyingspeed _normalflyingspeed)
        (set `self.CurrentFlyingSpeed` (- _currentflyingspeed _returnvalue_5))
        (else
          (set `self.CurrentFlyingSpeed` _normalflyingspeed))))
    ;[1 1 1] Calculate Flying Direction
    (bind _output_get_4 (set `self.FlyingDirection` (- (`SceneComponent.K2_GetComponentLocation` (`self.SpringArmLocalReferenceArrow`)) (`Actor.K2_GetActorLocation` (`self.Pawn`)))))
    (if (not (`self.HoverMode`))
      (set `self.FlyingDirection` (`KismetMathLibrary.MakeVector` (.x _output_get_4) (.y _output_get_4))))
    (set `self.FlyingDirection` (`KismetMathLibrary.Normal` (`self.FlyingDirection`)))
    ;[1 1 1] Displacement
    (bind _output_get_5 (set `self.FlyingSpeed` (* (`self.CurrentFlyingSpeed`) (`self.PowerFactor`) (`self.WeightFactor`))))
    (set `FloatingPawnMovement.MaxSpeed` _output_get_5 (`self.FloatingPawnMovement`))
    (bind _output_get_6 (set `self.FlyingVelocity` (* (`self.FlyingDirection`) _output_get_5)))
    (`Pawn.AddMovementInput` (`self.Pawn`) (* _output_get_6 (`GameplayStatics.GetWorldDeltaSeconds`)) 1.0 false)
    (set `self.FlyingDirection` (0.0 0.0 0.0))
    (else
      (`SceneComponent.K2_SetWorldRotation` _rollroot (`KismetMathLibrary.RLerp` (`SceneComponent.K2_GetComponentRotation` _rollroot) (`KismetMathLibrary.MakeRotator` 0.0 0.0 _returnvalue_yaw_2) (* (`self.MeshRollTurningRecoverySmoothingFactor`) _returnvalue_3) true) false false)
      (`SceneComponent.K2_SetRelativeRotation` _meshroot (`KismetMathLibrary.MakeRotator` 0.0 (`KismetMathLibrary.Lerp` _relativerotation_pitch 0.0 (* (`self.MeshPitchTurningRecoverySmoothingFactor`) _returnvalue_3))) false false))))

(fn `Land`
  (set `self.InAir` false))

(fn `SetAcceleration`
  (params (Value :type "Float (double-precision)"))
  (set `FloatingPawnMovement.Acceleration` Value (`self.FloatingPawnMovement`)))

(fn `SetDeceleration`
  (params (Value :type "Float (double-precision)"))
  (set `FloatingPawnMovement.Deceleration` Value (`self.FloatingPawnMovement`)))

(fn `SetMaximumSpeed`
  (params (Value :type "Float (double-precision)"))
  (set `FloatingPawnMovement.MaxSpeed` Value (`self.FloatingPawnMovement`)))

(fn `TakeOff`
  (set `self.InAir` true))